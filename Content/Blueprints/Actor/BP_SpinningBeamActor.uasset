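; BP_SpinningBeamActor is an actor that draws a Niagara beam from its owner to itself.
; On BeginPlay it spawns the beam system attached to the owner's root component.
; Each tick it writes its own location to the "Beam End" variable, so the beam follows the actor, and it destroys the Niagara component when the actor is destroyed.
; The spinning motion is not driven by these graphs.
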(event `self.ReceiveBeginPlay`
  (bind _returnvalue (`NiagaraFunctionLibrary.SpawnSystemAttached` (`self.BeamNiagara`) (`Actor.RootComponent` (`self.GetOwner`)) "None" (0.0 0.0 0.0) (struct) "SnapToTarget"))
  (set `self.Niagara` _returnvalue))

(event `self.ReceiveTick`
  (params (DeltaSeconds :type "Float (single-precision)"))
  (`NiagaraComponent.SetVariableVec3` (`self.Niagara`) "Beam End" (`self.K2_GetActorLocation`)))

(event `self.ReceiveDestroyed`
  (`ActorComponent.K2_DestroyComponent` (`self.Niagara`)))

(fn `UserConstructionScript`)