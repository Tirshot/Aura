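; Base pickup actor that plays a spawn animation with sound cues when it appears in the world.
; On BeginPlay, the Elevation timeline drives its height above the spawn point, multiplied by SpawnApex, along with its uniform scale.
; A DoOnce plays the ground impact sound when the elevation first dips below zero, and flags mark the animation's end.
; Destruction plays the consume sound; collection logic is absent here.
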(event `self.ReceiveBeginPlay`
  (bind _scale (`self.Scale`))
  (bind _output_get (set `self.InitialLocation` (`self.K2_GetActorLocation`)))
  (`GameplayStatics.PlaySoundAtLocation` (`self.SpawnSound`) _output_get (struct) 1.0 1.0 0.0 null null null null)
  (bind (_direction _elevation _scale_2) (`Timeline|Elevation`)
    (:`Update`
      (set `self.Elevation_Loc` _elevation)
      (set `self.Scale` _scale_2)
      (set `self.CalculatedLocation` (`self.CaculateElevation` (`self.Elevation_Loc`)))
      (`|ExecutionSequence`
        (:`then_0`
          (`self.K2_SetActorLocation` (`self.CalculatedLocation`)))
        (:`then_1`
          (`self.SetActorScale3D` (`KismetMathLibrary.MakeVector` _scale _scale _scale))
          (if (< (`self.Elevation_Loc`) 0.0)
            (`/Engine/EditorBlueprintResources/StandardMacros.DoOnce` false
              (:`Completed`
                (`GameplayStatics.PlaySoundAtLocation` (`self.GroundImpectSound`) (`self.K2_GetActorLocation`) (struct) 1.0 1.0 0.0 null null null null)))))))
    (:`Finished`
      (set `self.bAnimationFinished` true)
      (set `self.bAnimFinished` true))))

(event `self.ReceiveDestroyed`
  (`GameplayStatics.PlaySoundAtLocation` (`self.ConsumeSound`) (`self.K2_GetActorLocation`) (struct) 1.0 1.0 0.0 null null null null))

(event `self.ReceiveTick`
  (params (DeltaSeconds :type "Float (single-precision)")))

(fn `CaculateElevation`
  (params (Timeline :type "Float (double-precision)"))
  (returns (ReturnValue :type "Vector Structure"))
  (return (`KismetMathLibrary.MakeVector` (.x (`self.InitialLocation`)) (.y (`self.InitialLocation`)) (+ (.z (`self.InitialLocation`)) (* Timeline (`self.SpawnApex`))))))

(fn `UserConstructionScript`)