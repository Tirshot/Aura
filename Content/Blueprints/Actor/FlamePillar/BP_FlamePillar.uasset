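; Flame pillar actor whose fire light flickers continuously during play.
; From BeginPlay, it randomly picks one of two timelines, and each picks again when it finishes, so the flicker pattern varies.
; Each timeline's FlameIntensity track feeds ScaleFlameIntensity, which multiplies it by BaseIntensity to set the FireLight intensity.
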(event `Choose Timeline`
  (switch `int` (`KismetMathLibrary.RandomIntegerInRange` 0 1)
    (:`Default`
      (`self.ChooseTimeline_2` :!label _label))
    (:`0`
      (`self.ChooseTimeline_1`))
    (:`1`
      (goto _label))))

(event `self.ReceiveBeginPlay`
  (`self.Choose Timeline`))

(event `ChooseTimeline_1`
  (bind (_direction _flameintensity) (`Timeline|FlameIntensity` :!via `PlayFromStart`)
    (:`Update`
      (`self.Scale Flame Intensity` _flameintensity))
    (:`Finished`
      (`self.Choose Timeline`))))

(event `ChooseTimeline_2`
  (bind (_direction _flameintensity) (`Timeline|타임라인` :!via `PlayFromStart`)
    (:`Update`
      (`self.Scale Flame Intensity` _flameintensity))
    (:`Finished`
      (`self.Choose Timeline`))))

(fn `Scale Flame Intensity`
  (params (Intensity :type "Float (double-precision)"))
  (`LightComponent.SetIntensity` (`self.FireLight`) (* Intensity (`self.BaseIntensity`))))

(fn `UserConstructionScript`)