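; Checkpoint beacon that lights up and grants the player a staff item when reached.
; A sphere overlap by a PlayerInterface actor calls HandleGlowEffects, sets Reached, and has AuraGameModeBase give the hardcoded item to player 0's character.
; The CheckPointReached event plays the Beacon timeline to drive the dynamic material's Glow parameter, scaled by GlowFactor.
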(event `self.CheckPointReached`
  (params (DynamicMI :type "MaterialInstanceDynamic Object Reference") (InteractedActor :type "Actor Object Reference"))
  (bind (_direction _beacon) (`Timeline|Beacon`)
    (:`Update`
      (`MaterialInstanceDynamic.SetScalarParameterValue` DynamicMI "Glow" (* _beacon (`self.GlowFactor`))))))

(event `self.Sphere.OnComponentBeginOverlap`
  (params (OverlappedComponent :type "PrimitiveComponent Object Reference") (OtherActor :type "Actor Object Reference") (OtherComp :type "PrimitiveComponent Object Reference") (OtherBodyIndex :type Integer) (bFromSweep :type Boolean) (SweepResult :type "HitResult Structure (by ref)"))
  (if (`KismetSystemLibrary.DoesImplementInterface` OtherActor "/Script/Aura.PlayerInterface")
    (`self.HandleGlowEffects` null)
    (set `self.bReached` true)
    (bind _asaura_game_mode_base (cast `AuraGameModeBase` (`GameplayStatics.GetGameMode`)))
    (bind _asaura_character (cast `AuraCharacter` (`GameplayStatics.GetPlayerCharacter` 0)))
    (`AuraGameModeBase.GiveItemToCharacter` _asaura_game_mode_base _asaura_character "Staff_002" 1)))

(fn `UserConstructionScript`)