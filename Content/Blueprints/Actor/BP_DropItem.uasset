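; BP_DropItem is a dropped item actor with a name widget that briefly labels it in the world.
; When OnDropItemInitialized fires, it fills the widget with title, rarity, count and stackability from DropItemData.
; A timeline then animates the drop by setting absolute world Z and roll, sweeping the movement.
; A timer started at BeginPlay hides the name, and cursor hover recolors the label background.
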(event `self.ReceiveBeginPlay`
  (add `self.OnDropItemInitialized` (delegate `OnDropItemInitialized_이벤트`))
  (`KismetSystemLibrary.K2_SetTimerDelegate` (delegate `HideItemName`) 5.0))

(event `OnDropItemInitialized_이벤트` :!signature `self.OnDropItemInitialized`
  (params (ItemTitle :type Text))
  (bind (_returnvalue_roll _returnvalue_pitch _returnvalue_yaw) (`KismetMathLibrary.BreakRotator` (`self.K2_GetActorRotation`)))
  (bind (_returnvalue_x _returnvalue_y) (`KismetMathLibrary.BreakVector` (`self.K2_GetActorLocation`)))
  (bind (_uniqueid _name _displayname _size _bstackable _itemcounts _image _staticmesh _leftfootmesh _rightfootmesh _material _description _itemstat _effectandstacks _abilitytagandlevel _abilityupgradetagandlevel _rarity) (break `ItemData` (`self.DropItemData`)))
  (`|ExecutionSequence`
    (:`then_0`
      (bind _asbp_drop_item_name (cast `/Game/Blueprints/UI/InventoryMenu/BP_DropItemName` (`WidgetComponent.GetWidget` (`self.ItemTitleWidget`))))
      (`/Game/Blueprints/UI/InventoryMenu/BP_DropItemName.SetItemName` _asbp_drop_item_name ItemTitle _rarity _itemcounts _bstackable)
      (set `self.InitialLocation` (`self.K2_GetActorLocation`))
      (set `self.InitialRotation` (`self.K2_GetActorRotation`)))
    (:`then_1`
      (bind (_direction `_새_트랙_0` _rotate) (`Timeline|타임라인`)
        (:`Update`
          (`self.K2_SetActorLocation` (`KismetMathLibrary.MakeVector` _returnvalue_x _returnvalue_y (* `_새_트랙_0` 350.0)) true)
          (`self.K2_SetActorRotation` (`KismetMathLibrary.MakeRotator` _rotate _returnvalue_pitch _returnvalue_yaw)))
        (:`Finished`
          (`self.K2_SetActorLocation` (`self.K2_GetActorLocation`) true))))))

(event `HideItemName`
  (`SceneComponent.SetVisibility` (`self.ItemTitleWidget`) false false))

(event `self.ItemTitleWidget.OnBeginCursorOver`
  (params (TouchedComponent :type "PrimitiveComponent Object Reference"))
  (bind `_as위젯_컴포넌트` (cast `WidgetComponent` TouchedComponent))
  (bind _asbp_drop_item_name (cast `/Game/Blueprints/UI/InventoryMenu/BP_DropItemName` (`WidgetComponent.GetWidget` `_as위젯_컴포넌트`)))
  (`Image.SetColorAndOpacity` (`/Game/Blueprints/UI/InventoryMenu/BP_DropItemName.Image_Background` _asbp_drop_item_name) (struct :`G` 0.182202 :`B` 1.0 :`A` 0.8)))

(event `self.ItemTitleWidget.OnEndCursorOver`
  (params (TouchedComponent :type "PrimitiveComponent Object Reference"))
  (bind _asbp_drop_item_name (cast `/Game/Blueprints/UI/InventoryMenu/BP_DropItemName` (`WidgetComponent.GetWidget` (`self.ItemTitleWidget`))))
  (`Image.SetColorAndOpacity` (`/Game/Blueprints/UI/InventoryMenu/BP_DropItemName.Image_Background` _asbp_drop_item_name) (struct :`A` 0.2)))

(fn `UserConstructionScript`)