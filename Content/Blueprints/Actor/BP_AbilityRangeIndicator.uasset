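; BP_AbilityRangeIndicator is a decal actor that shows an ability's range, attached to the avatar actor.
; BeginPlay creates a dynamic decal material and binds the IndicatorInitialized event.
; That event attaches the actor, offsets its height using a visibility trace around the world origin, scales it by Radius and sets the outline color.
; RangeShape, Location, Width and Height are unused.
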(event `self.ReceiveBeginPlay`
  (bind _returnvalue (`DecalComponent.CreateDynamicMaterialInstance` (`self.DecalComponent`)))
  (set `self.DynamicMaterialInst` _returnvalue)
  (add `self.IndicatorInitialized` (delegate `IndicatorInitialized_이벤트`)))

(event `IndicatorInitialized_이벤트` :!signature `self.IndicatorInitialized`
  (params (AvatarActor :type "Actor Object Reference") (RangeShape :type "ERangeShape Enum" :default "ERS_Circle") (Location :type "Vector Structure (by ref)") (Width :type "Float (single-precision)") (Height :type "Float (single-precision)") (Radius :type "Float (single-precision)") (Red :type "Float (single-precision)") (Green :type "Float (single-precision)") (Blue :type "Float (single-precision)"))
  (set `self.Radius` Radius)
  (set `self.Red` Red)
  (set `self.Green` Green)
  (set `self.Blue` Blue)
  (`self.K2_AttachToActor` AvatarActor "None" "KeepRelative" "KeepRelative" "KeepWorld")
  (bind _outhit (`KismetSystemLibrary.LineTraceSingle` (0.0 0.0 -300.0) (0.0 0.0 300.0) "TraceTypeQuery1" false (`|MakeArray` AvatarActor)))
  (`self.K2_AddActorWorldOffset` (`KismetMathLibrary.MakeVector` 0.0 0.0 (* (.z (`.Location` (`GameplayStatics.BreakHitResult` _outhit))) 2.0)))
  (bind _output_get (set `self.Scale` (/ (`self.Radius`) 100.0)))
  (`self.SetActorScale3D` (`KismetMathLibrary.MakeVector` 1.0 _output_get _output_get))
  (`MaterialInstanceDynamic.SetVectorParameterValue` (`self.DynamicMaterialInst`) "OutlineColor" (make `LinearColor` (/ (`self.Red`) 100.0) (/ (`self.Green`) 100.0) (/ (`self.Blue`) 100.0) 0.12)))

(fn `UserConstructionScript`)