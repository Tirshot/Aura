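; Actor whose mesh fades out and back in through a timeline-driven "Fade" material parameter.
; The construction script caches original materials and builds dynamic instances from FadeMaterialInstances, which FadeOut swaps in by slot before playing the timeline; Fadein reverses it.
; When the timeline finishes, a value of one restores original materials and blocking collision, while zero ignores a custom trace channel, plus Visibility if BlockVisiblity is set.
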(event `/Game/Blueprints/Actor/FadeActor/BI_FadeInterface.FadeOut`
  (`self.Set Materials to Dynamic Instances`)
  (bind (_direction _fade) (`Timeline|FadeTimeline` :!via `PlayFromStart` :!label _label)
    (:`Update`
      (for _array_element (`self.DynamicMatrialInstances`)
        (`MaterialInstanceDynamic.SetScalarParameterValue` _array_element "Fade" _fade)))
    (:`Finished`
      (bind _output_get (set `self.FinalFadeValue` _fade))
      (`self.FadeFinished` _output_get))))

(event `/Game/Blueprints/Actor/FadeActor/BI_FadeInterface.FadeIn`
  (goto _label :!via `Reverse`))

(event `self.ReceiveBeginPlay`)

(fn `FadeFinished`
  (params (Fade :type "Float (double-precision)"))
  (if (>= Fade 1.0)
    (`self.Reset Materials`)
    (`PrimitiveComponent.SetCollisionResponseToChannel` (`self.Mesh`) "ECC_GameTraceChannel2" "ECR_Block")
    (if (`self.BlockVisiblity`)
      (`PrimitiveComponent.SetCollisionResponseToChannel` (`self.Mesh`) "ECC_Visibility" "ECR_Block"))
    (elif (<= Fade 0.0)
      (`PrimitiveComponent.SetCollisionResponseToChannel` (`self.Mesh`) "ECC_GameTraceChannel2" "ECR_Ignore")
      (if (`self.BlockVisiblity`)
        (`PrimitiveComponent.SetCollisionResponseToChannel` (`self.Mesh`) "ECC_Visibility" "ECR_Ignore")))))

(fn `Reset Materials`
  (for (_array_element _array_index) (`self.OriginalMaterials`)
    (`PrimitiveComponent.SetMaterial` (`self.Mesh`) _array_index _array_element)))

(fn `Set Materials to Dynamic Instances`
  (for (_array_element _array_index) (`self.DynamicMatrialInstances`)
    (`PrimitiveComponent.SetMaterial` (`self.Mesh`) _array_index _array_element)))

(fn `UserConstructionScript`
  (`KismetArrayLibrary.Array_Clear` (`self.DynamicMatrialInstances`))
  (set `self.OriginalMaterials` (`MeshComponent.GetMaterials` (`self.Mesh`)))
  (for _array_element (`self.FadeMaterialInstances`)
    (bind _returnvalue (`KismetMaterialLibrary.CreateDynamicMaterialInstance` _array_element))
    (`KismetArrayLibrary.Array_AddUnique` (`self.DynamicMatrialInstances`) _returnvalue)))