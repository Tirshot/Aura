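; Enemy gameplay ability for the Shaman's spinning lightning beam attack.
; On activation it teleports the avatar to a hardcoded XY spot and plays the montage from its Loop section.
; One gameplay event spawns rotating rectangular range indicators evenly around the avatar, one per beam; another calls SpawnBeam, which is not defined in this graph.
; Cooldown is committed only when BeamDestroyed fires, which also ends the ability.
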(event `self.K2_ActivateAbility`
  (bind _returnvalue (`self.GetAvatarActorFromActorInfo`))
  (bind (_returnvalue_x _returnvalue_y _returnvalue_z) (`KismetMathLibrary.BreakVector` (`Actor.K2_GetActorLocation` _returnvalue)))
  (bind _returnvalue_2 (`Actor.K2_GetActorRotation` (`self.GetAvatarActorFromActorInfo`)))
  (`Actor.K2_SetActorLocation` _returnvalue (`KismetMathLibrary.MakeVector` -415.45166 -295.444214 _returnvalue_z) false false)
  (`AbilityTask_PlayMontageAndWait.CreatePlayMontageAndWaitProxy` "None" "/Game/Assets/Enemies/Shaman/Animations/AM_Shaman_SpinningBeam.AM_Shaman_SpinningBeam" 1.0 "Loop"
    (:`then`
      (`|ExecutionSequence`
        (:`then_0`
          (`AbilityTask_WaitGameplayEvent.WaitGameplayEvent` (struct :`TagName` "Event.RangeIndicator") null true
            (:`EventReceived`
              (for _array_element (`AuraAbilitySystemLibrary.EvenlySpacedRotators` (`KismetMathLibrary.GetForwardVector` _returnvalue_2) (`KismetMathLibrary.GetUpVector` _returnvalue_2) 360.0 (`self.BeamCount`))
                (bind _returnvalue_3 (`self.SpawnRangeIndicator` (`Actor.K2_GetActorLocation` (`self.GetAvatarActorFromActorInfo`)) false "ERS_Rectangle" 0.0 30.0 (`self.OrbitRadius`) (0.0 0.0 0.0) 1.0))
                (`Actor.K2_SetActorRotation` _returnvalue_3 _array_element false)
                (set `AbilityRangeIndicator.bRotate` true _returnvalue_3)
                (set `AbilityRangeIndicator.RotationSpeed` 30.0 _returnvalue_3)))))
        (:`then_1`
          (`AbilityTask_WaitGameplayEvent.WaitGameplayEvent` (struct :`TagName` "Abilities.Lightning.SpinningBeam") null true
            (:`EventReceived`
              (`self.SpawnBeam`))))))))

(event `self.BeamDestroyed`
  (`self.K2_CommitAbilityCooldown` false true)
  (`self.K2_EndAbility`))