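; Enemy gameplay ability that casts a fire tornado at the location of the AI's blackboard target.
; On activation it snapshots the target location, turns the avatar toward it, and plays the Shaman FireNado montage while showing a circular damage-radius indicator there.
; The Firenado gameplay event triggers the tornado spawn and commits the cooldown.
; This graph ends the ability only on montage interruption or cancellation.
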(event `self.K2_ActivateAbility`
  (`parent.K2_ActivateAbility`)
  (set `self.Target` (`BlackboardComponent.GetValueAsObject` (`AIBlueprintHelperLibrary.GetBlackboard` (`self.GetAvatarActorFromActorInfo`)) (`self.TargetKey`)))
  (`|ExecutionSequence`
    (:`then_0`
      (bind `_as액터` (cast `Actor` (`self.Target`)))
      (set `self.TargetLocation` (`Actor.K2_GetActorLocation` `_as액터`))
      (`self.UpdateFacingTarget`))
    (:`then_1`
      (`AbilityTask_PlayMontageAndWait.CreatePlayMontageAndWaitProxy` "None" "/Game/Assets/Enemies/Shaman/Animations/AM_Shaman_FireNado.AM_Shaman_FireNado"
        (:`then`
          (`self.SpawnRangeIndicator` (`self.TargetLocation`) false "ERS_Circle" (`self.DamageRadius`) 0.0 0.0 (0.0 0.0 0.0) 1.5)
          (`AbilityTask_WaitGameplayEvent.WaitGameplayEvent` (struct :`TagName` "Abilities.Fire.Firenado") null true
            (:`EventReceived`
              (`self.SpawnTornadoToLocation` (`self.TargetLocation`))
              (`self.K2_CommitAbilityCooldown` false))))
        (:`OnInterrupted`
          (`self.K2_EndAbility` :!label _label))
        (:`OnCancelled`
          (goto _label))))))

(fn `UpdateFacingTarget`
  (message `CombatInterface.UpdateFacingTarget` (`self.GetAvatarActorFromActorInfo`) (`self.TargetLocation`)))