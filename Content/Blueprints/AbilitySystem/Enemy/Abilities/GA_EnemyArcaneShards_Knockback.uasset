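; Enemy Gameplay Ability for the shaman's Arcane Shards knockback attack, aimed at the blackboard target if it implements CombatInterface.
; On activation it caches the target location, updates the motion-warping facing, creates a point collection and plays the cast montage.
; Gameplay events then trigger range indicators and the shard spawn, each once.
; It ends immediately if the target is not an Actor.
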(event `self.K2_ActivateAbility`
  (`parent.K2_ActivateAbility`)
  (`self.CheckAbilityUpgrades`)
  (bind _output_get (set `self.Target` (`BlackboardComponent.GetValueAsObject` (`AIBlueprintHelperLibrary.GetBlackboard` (`self.GetAvatarActorFromActorInfo`)) (`self.TargetKey`))))
  (bind `_as액터` (cast `Actor` _output_get)
    (:`then`
      (if (`KismetSystemLibrary.DoesImplementInterface` `_as액터` "/Script/Aura.CombatInterface")
        (set `self.CurrentTargetLocation` (`Actor.K2_GetActorLocation` `_as액터`))
        (`|ExecutionSequence`
          (:`then_0`
            ;[1 1 1] 모션 워핑
            (message `CombatInterface.UpdateFacingTarget` (`self.GetAvatarActorFromActorInfo`) (`self.CurrentTargetLocation`))
            (`self.CreatePointCollection`))
          (:`then_1`
            ;[1 1 1] 몽타주 재생 대기
            (`AbilityTask_PlayMontageAndWait.CreatePlayMontageAndWaitProxy` "None" "/Game/Assets/Enemies/Shaman/Animations/AM_Shaman_ArcaneShards.AM_Shaman_ArcaneShards" 1.0 "None" true 1.0 0.0 true
              (:`then`
                (`AbilityTask_WaitGameplayEvent.WaitGameplayEvent` (struct :`TagName` "Event.RangeIndicator") null true
                  (:`EventReceived`
                    (`self.SpawnRangeIndicators`))))))
          (:`then_2`
            (`AbilityTask_WaitGameplayEvent.WaitGameplayEvent` (struct :`TagName` "Abilities.Arcane.ArcaneShards") null true
              (:`EventReceived`
                (`self.ReadyToSpawnShards`)))))))
    (:`CastFailed`
      (`self.K2_EndAbility`))))

(event `self.K2_OnEndAbility`
  (params (bWasCancelled :type Boolean))
  (`parent.K2_OnEndAbility` bWasCancelled))