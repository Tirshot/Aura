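; Enemy gameplay ability (shaman summon montage) that spawns random minions at shuffled spawn locations.
; On activation it shows ground Niagara effects at every location and plays the montage, then waits for the Abilities.Summon event.
; That event starts a delayed loop spawning GAS minions slightly above ground, two levels below the ability, with default controllers.
; The avatar's minion count and list are updated on each spawn and destruction.
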(event `self.K2_ActivateAbility`
  (bind _returnvalue (`self.GetAvatarActorFromActorInfo`))
  (bind _returnvalue_2 (`self.GetAvatarActorFromActorInfo`))
  (bind _returnvalue_3 (+ (`|GetArrayItem` (`self.SpawnLocations`) (`self.SpawnLocationIndex`)) (0.0 0.0 70.0)))
  (bind _returnvalue_4 (`self.GetSpawnLocations`))
  (bind _output_get (set `self.SpawnLocations` _returnvalue_4))
  (`KismetArrayLibrary.Array_Shuffle` _output_get)
  (for _array_element _output_get
    (`NiagaraFunctionLibrary.SpawnSystemAtLocation` "/Game/Assets/Effects/Combat/NS_GroundSummon.NS_GroundSummon" _array_element))
  (`AbilityTask_PlayMontageAndWait.CreatePlayMontageAndWaitProxy` "None" "/Game/Assets/Enemies/Shaman/Animations/AM_Shaman_Summon.AM_Shaman_Summon"
    (:`then`
      (`AbilityTask_WaitGameplayEvent.WaitGameplayEvent` (struct :`TagName` "Abilities.Summon") null
        (:`EventReceived`
          (if (< (`self.SpawnLocationIndex`) (`KismetArrayLibrary.Array_Length` (`self.SpawnLocations`))) :!label _label
            (bind _returnvalue_5 (`AuraAbilitySystemLibrary.SpawnGASActor` _returnvalue (`self.GetRandomMinionClass`) (- (`self.GetAbilityLevel`) 2) (`KismetMathLibrary.MakeTransform` _returnvalue_3 (`KismetMathLibrary.FindLookAtRotation` (`Actor.K2_GetActorLocation` (`self.GetAvatarActorFromActorInfo`)) _returnvalue_3)) _returnvalue))
            (bind _output_get_2 (set `self.SpawnedMinion` _returnvalue_5))
            (add `Actor.OnDestroyed` _output_get_2 (delegate `OnDestroyed_이벤트`))
            (`Pawn.SpawnDefaultController` (`self.SpawnedMinion`))
            (message `CombatInterface.IncrementMinionCount` _returnvalue_2 1)
            (bind _asaura_character_base (cast `AuraCharacterBase` _returnvalue_2))
            (`KismetArrayLibrary.Array_AddUnique` (`AuraCharacterBase.Minions` _asaura_character_base) (`self.SpawnedMinion`))
            (`/Engine/EditorBlueprintResources/StandardMacros.IncrementInt` (`self.SpawnLocationIndex`)
              (:`  `
                (`KismetSystemLibrary.Delay` 0.05)
                (goto _label)))
            (else
              (`self.K2_EndAbility`))))))))

(event `self.K2_OnEndAbility`
  (params (bWasCancelled :type Boolean))
  (set `self.SpawnLocationIndex` 0)
  (`KismetArrayLibrary.Array_Clear` (`self.SpawnLocations`)))

(event `OnDestroyed_이벤트`
  (params (DestroyedActor :type "Actor Object Reference"))
  (bind _returnvalue (`self.GetAvatarActorFromActorInfo`))
  (message `CombatInterface.IncrementMinionCount` _returnvalue -1)
  (bind _asaura_character_base (cast `AuraCharacterBase` _returnvalue))
  (`KismetArrayLibrary.Array_RemoveItem` (`AuraCharacterBase.Minions` _asaura_character_base) DestroyedActor))