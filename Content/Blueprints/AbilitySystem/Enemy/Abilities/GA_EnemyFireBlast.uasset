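; Enemy gameplay ability that fires a radial burst of fireballs, telegraphed with range indicators.
; On activation it commits, then spawns short-lived rectangular indicators around the avatar along evenly spaced rotators, one per NumFireBalls.
; After a brief delay it calls SpawnFireBalls, marks each returned fireball's ApexLocation with a circular indicator, and ends immediately.
; Spawning logic and fireball movement are defined outside this graph.
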(event `self.K2_ActivateAbility`
  (bind _returnvalue (`Actor.K2_GetActorRotation` (`self.GetAvatarActorFromActorInfo`)))
  (`self.K2_CommitAbility`)
  (for _array_element (`AuraAbilitySystemLibrary.EvenlySpacedRotators` (`KismetMathLibrary.GetForwardVector` _returnvalue) (`KismetMathLibrary.GetUpVector` _returnvalue) 360.0 (`self.NumFireBalls`))
    (bind _returnvalue_2 (`self.SpawnRangeIndicator` (`Actor.K2_GetActorLocation` (`self.GetAvatarActorFromActorInfo`)) false "ERS_Rectangle" 0.0 30.0 600.0 (`self.RangeIndicatorRGB`) 1.0))
    (`Actor.K2_SetActorRotation` _returnvalue_2 _array_element false))
  (`KismetSystemLibrary.Delay` 0.5)
  (bind _returnvalue_3 (`self.SpawnFireBalls`))
  (for _array_element_2 _returnvalue_3
    (`self.SpawnRangeIndicator` (`AuraFireBall.ApexLocation` _array_element_2) false "ERS_Circle" 50.0 30.0 600.0 (`self.RangeIndicatorRGB`) 2.0))
  (`self.K2_EndAbility`))