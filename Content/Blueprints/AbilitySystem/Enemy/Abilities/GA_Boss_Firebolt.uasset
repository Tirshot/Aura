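; Gameplay ability for a boss that casts homing firebolts at the target actor stored in its AI blackboard.
; It turns the avatar toward the target, plays the shaman firebolt montage and waits for a gameplay event to spawn projectiles from the weapon socket with a pitch override.
; The blackboard berserk flag raises the projectile count, and the ability ends after spawning or on montage interruption or cancellation.
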(event `self.K2_ActivateAbility`
  (bind `_as액터` (cast `Actor` (`BlackboardComponent.GetValueAsObject` (`AIBlueprintHelperLibrary.GetBlackboard` (`self.GetAvatarActorFromActorInfo`)) (`self.TargetKey`))))
  (bind _output_get (set `self.TargetActor` `_as액터`))
  (bind _output_get_2 (set `self.ProjectileTargetLocation` (`Actor.K2_GetActorLocation` _output_get)))
  (message `CombatInterface.UpdateFacingTarget` (`self.GetAvatarActorFromActorInfo`) _output_get_2)
  (`AbilityTask_PlayMontageAndWait.CreatePlayMontageAndWaitProxy` "None" "/Game/Assets/Enemies/Shaman/Animations/AM_Shaman_FireBolt.AM_Shaman_FireBolt" 1.0 "None" false
    (:`then`
      (`AbilityTask_WaitGameplayEvent.WaitGameplayEvent` (struct :`TagName` "Abilities.Fire.FireBolt") null true
        (:`EventReceived`
          (if (`BlackboardComponent.GetValueAsBool` (`AIBlueprintHelperLibrary.GetBlackboard` (`self.GetAvatarActorFromActorInfo`)) (`self.BerserkKey`))
            (`self.SpawnProjectiles` (`self.ProjectileTargetLocation`) (`BlueprintGameplayTagLibrary.MakeLiteralGameplayTag` (struct :`TagName` "CombatSocket.Weapon")) true 15.0 true 3 (`self.TargetActor`))
            (else
              (`self.SpawnProjectiles` (`self.ProjectileTargetLocation`) (`BlueprintGameplayTagLibrary.MakeLiteralGameplayTag` (struct :`TagName` "CombatSocket.Weapon")) true 15.0 true 2 (`self.TargetActor`))))
          (`self.K2_EndAbility`))))
    (:`OnInterrupted`
      (`self.K2_EndAbility` :!label _label))
    (:`OnCancelled`
      (goto _label))))