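; Enemy gameplay ability for a shaman's cone of rotating beams, aimed at the player character stored in the AI blackboard.
; It warps facing toward the target and plays the spinning-beam montage, whose gameplay events trigger telegraphs and SpawnBeam.
; Evenly spread rectangular range indicators rotate with a lifespan equal to the time to sweep the spread angle.
; BeamDestroyed commits the cooldown and ends the ability.
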(event `self.K2_ActivateAbility`
  (bind _asbp_aura_character (cast `/Game/Blueprints/Character/Aura/BP_AuraCharacter` (`BlackboardComponent.GetValueAsObject` (`AIBlueprintHelperLibrary.GetBlackboard` (`self.GetAvatarActorFromActorInfo`)) (`self.TargetKey`))))
  (set `self.Target` _asbp_aura_character)
  ;[1 1 1] 모션 워핑
  (message `CombatInterface.UpdateFacingTarget` (`self.GetAvatarActorFromActorInfo`) (`self.CurrentTargetLocation`))
  (`AbilityTask_PlayMontageAndWait.CreatePlayMontageAndWaitProxy` "None" "/Game/Assets/Enemies/Shaman/Animations/AM_Shaman_SpinningBeam.AM_Shaman_SpinningBeam" 1.0 "Loop"
    (:`then`
      (`|ExecutionSequence`
        (:`then_0`
          (`AbilityTask_WaitGameplayEvent.WaitGameplayEvent` (struct :`TagName` "Event.RangeIndicator") null true
            (:`EventReceived`
              (bind _output_get (set `self.SavedRotators` (`AuraAbilitySystemLibrary.EvenlySpacedRotators` (`KismetMathLibrary.GetForwardVector` (`KismetMathLibrary.MakeRotator` (.roll (`Actor.K2_GetActorRotation` (`self.GetAvatarActorFromActorInfo`))) (.pitch (`Actor.K2_GetActorRotation` (`self.GetAvatarActorFromActorInfo`))) (- (.yaw (`Actor.K2_GetActorRotation` (`self.GetAvatarActorFromActorInfo`))) (/ (`self.SpreadDegree`) 2.0)))) (`KismetMathLibrary.GetUpVector` (`Actor.K2_GetActorRotation` (`self.GetAvatarActorFromActorInfo`))) (`self.SpreadDegree`) (`self.BeamCount`))))
              (for _array_element _output_get
                (bind _returnvalue (`self.SpawnRangeIndicator` (`Actor.GetActorUpVector` (`self.GetAvatarActorFromActorInfo`)) true "ERS_Rectangle" 0.0 30.0 (`self.OrbitRadius`) (0.0 0.0 0.0) (/ (`self.SpreadDegree`) (`self.AngleSpeed`))))
                (`Actor.K2_SetActorRotation` _returnvalue _array_element false)
                (set `AbilityRangeIndicator.bRotate` true _returnvalue)
                (set `AbilityRangeIndicator.RotationSpeed` (`self.AngleSpeed`) _returnvalue)))))
        (:`then_1`
          (`AbilityTask_WaitGameplayEvent.WaitGameplayEvent` (struct :`TagName` "Abilities.Lightning.SpinningBeam") null true
            (:`EventReceived`
              (`self.SpawnBeam`))))))))

(event `self.BeamDestroyed`
  (`self.K2_CommitAbilityCooldown` false true)
  (`self.K2_EndAbility`))