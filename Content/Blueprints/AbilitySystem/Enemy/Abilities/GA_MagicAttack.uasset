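; GA_MagicAttack is an enemy gameplay ability that makes its owner cast a fire bolt projectile at its combat target.
; On activation it turns the avatar toward the target and plays the shaman FireBolt montage.
; A one-shot gameplay event then triggers SpawnProjectile from the weapon socket toward the target's current location, with optional pitch override.
; It then commits the cooldown and ends the ability.
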(event `self.K2_ActivateAbility`
  (bind _returnvalue (`self.GetAvatarActorFromActorInfo`))
  (bind _returnvalue_2 (message `EnemyInterface.GetCombatTarget` _returnvalue))
  (message `CombatInterface.UpdateFacingTarget` _returnvalue (`Actor.K2_GetActorLocation` _returnvalue_2))
  (`AbilityTask_PlayMontageAndWait.CreatePlayMontageAndWaitProxy` "None" "/Game/Assets/Enemies/Shaman/Animations/AM_Shaman_FireBolt.AM_Shaman_FireBolt" 1.0 "None" false
    (:`then`
      (`AbilityTask_WaitGameplayEvent.WaitGameplayEvent` (struct :`TagName` "Abilities.Fire.FireBolt") null true
        (:`EventReceived`
          (bind _returnvalue_3 (message `EnemyInterface.GetCombatTarget` (`self.GetAvatarActorFromActorInfo`)))
          (`self.SpawnProjectile` (`Actor.K2_GetActorLocation` _returnvalue_3) (`BlueprintGameplayTagLibrary.MakeLiteralGameplayTag` (struct :`TagName` "CombatSocket.Weapon")) (`self.Should Override Pitch`) (`self.Pitch Override`))
          (`self.K2_CommitAbilityCooldown` true)
          (`self.K2_EndAbility`))))))