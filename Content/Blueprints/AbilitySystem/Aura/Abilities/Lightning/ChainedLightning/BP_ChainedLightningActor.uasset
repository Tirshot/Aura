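; Visual actor for the chained lightning ability that draws an electric beam between two scene components, CueStart and CueEnd.
; On BeginPlay it spawns the chained-beam Niagara system attached to CueStart with auto-activation off, setting both endpoints before activating it.
; Tick rewrites the Beam Start and Beam End parameters from the components' world locations, so the beam follows them.
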(event `self.ReceiveBeginPlay`
  (bind _newvar (`self.NewVar`))
  (bind _returnvalue (`NiagaraFunctionLibrary.SpawnSystemAttached` "/Game/Assets/Effects/Shock/NS_ElectricBeam_Chained.NS_ElectricBeam_Chained" (`self.CueStart`) "None" (0.0 0.0 0.0) (struct) "KeepWorldPosition" false false))
  (set `self.NewVar` _returnvalue)
  (`NiagaraComponent.SetVariableVec3` _newvar "Beam Start" (`SceneComponent.K2_GetComponentLocation` (`self.CueStart`)))
  (`NiagaraComponent.SetVariableVec3` _newvar "Beam End" (`SceneComponent.K2_GetComponentLocation` (`self.CueEnd`)))
  (`ActorComponent.Activate` (`self.NewVar`) true))

(event `self.ReceiveTick`
  (params (DeltaSeconds :type "Float (single-precision)"))
  (bind _newvar (`self.NewVar`))
  (`NiagaraComponent.SetVariableVec3` _newvar "Beam Start" (`SceneComponent.K2_GetComponentLocation` (`self.CueStart`)))
  (`NiagaraComponent.SetVariableVec3` _newvar "Beam End" (`SceneComponent.K2_GetComponentLocation` (`self.CueEnd`))))

(fn `UserConstructionScript`)