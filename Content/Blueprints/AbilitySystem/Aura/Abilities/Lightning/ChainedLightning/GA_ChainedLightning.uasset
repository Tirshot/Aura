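; Gameplay ability for Aura's Chained Lightning that fires a projectile at the location under the mouse.
; On activation it checks upgrades, takes cursor target data, turns the caster toward the hit actor and plays the Electrocute cast montage.
; On montage notify or completion, the authority spawns the projectile using the spine socket tag with pitch override, then ends the ability, while non-authority ends it locally.
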(event `self.K2_ActivateAbility`
  (`self.CheckAbilityUpgrades`)
  (bind (_asynctaskproxy _datahandle) (`TargetDataUnderMouse.CreateTargetDataUnderMouse`)
    (:`ValidData`
      (bind (_bblockinghit _binitialoverlap _time _distance _location _impactpoint _normal _impactnormal _physmat _hitactor) (`GameplayStatics.BreakHitResult` (`AbilitySystemBlueprintLibrary.GetHitResultFromTargetData` _datahandle)))
      (if _bblockinghit
        (set `self.TargetLocation` _location)
        (bind _output_get (set `self.TargetActor` _hitactor))
        (message `CombatInterface.UpdateFacingTarget` (`self.GetAvatarActorFromActorInfo`) (`Actor.K2_GetActorLocation` _output_get))
        (bind _asbp_aura_character (cast `/Game/Blueprints/Character/Aura/BP_AuraCharacter` (`self.GetAvatarActorFromActorInfo`))
          (:`then`
            (`|PlayMontage` (`Character.Mesh` _asbp_aura_character) "/Game/Assets/Characters/Aura/Animations/Abilities/AM_Cast_Electrocute.AM_Cast_Electrocute"
              (:`OnCompleted`
                (`self.K2_HasAuthority` :!label _label
                  (:`True`
                    (`self.SpawnProjectile` (`self.TargetLocation`) (`BlueprintGameplayTagLibrary.MakeLiteralGameplayTag` (struct :`TagName` "CombatSocket.Spine")) true)
                    (`self.K2_EndAbility`))
                  (:`False`
                    (`self.K2_EndAbilityLocally`))))
              (:`OnInterrupted`
                (`self.K2_EndAbility` :!label _label_2))
              (:`OnNotifyBegin`
                (goto _label))))
          (:`CastFailed`
            (goto _label_2)))
        (else
          (`self.K2_EndAbility`))))))