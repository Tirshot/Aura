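; Aura lightning ability that places a temporary electrosphere at a targeted location to damage actors overlapping it.
; Input press under a magic circle and range indicator sets the target and plays the cast montage.
; The montage event spawns the sphere, then commits cost and cooldown.
; A looping timer applies damage, while a lifetime timer removes shock states and cues, destroys the sphere and ends the ability.
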(event `self.K2_ActivateAbility`
  (`self.ShowMagicCircle` (`self.DamageRadius`))
  (`self.ShowRangeIndicator` "ERS_Rectangle" 50.0)
  (`AbilityTask_WaitInputPress.WaitInputPress` false
    (:`OnPress`
      (bind (_asynctaskproxy _datahandle) (`TargetDataUnderMagicCircle.CreateTargetDataUnderMagicCircle`)
        (:`ValidData`
          (bind _returnvalue (`self.ReceivedMouseHitResult` _datahandle))
          (`self.HideMagicCircleAndRangeIndicator`)
          (message `CombatInterface.UpdateFacingTarget` (`self.GetAvatarActorFromActorInfo`) _returnvalue)
          (`GameplayCueFunctionLibrary.ExecuteGameplayCueOnActor` (`self.GetAvatarActorFromActorInfo`) (struct :`TagName` "GameplayCue.ElectroSphere.Spawn") (`AbilitySystemBlueprintLibrary.MakeGameplayCueParameters` 0.0))
          (`AbilityTask_PlayMontageAndWait.CreatePlayMontageAndWaitProxy` "None" "/Game/Assets/Characters/Aura/Animations/Abilities/AM_Cast_SpawnElectroSphere.AM_Cast_SpawnElectroSphere" 1.0 "None" false
            (:`then`
              (`AbilityTask_WaitGameplayEvent.WaitGameplayEvent` (struct :`TagName` "Event.Montage.SpawnElectroSphere") null true
                (:`EventReceived`
                  (`self.SpawnElectroSphere` (`self.MouseLocation`))
                  (`self.StopAutoRun`)
                  (`self.K2_CommitAbilityCost` false)
                  (`self.K2_CommitAbilityCooldown` false)
                  (`self.CheckAbilityUpgrades`)
                  (bind _electrosphere (`self.ElectroSphere`)
                    (:`then`
                      (`|ExecutionSequence`
                        (:`then_0`
                          (bind _returnvalue_2 (`KismetSystemLibrary.K2_SetTimerDelegate` (delegate `DestroySphere`) (`self.SpawnTime`)))
                          (set `self.Timer` _returnvalue_2))
                        (:`then_1`
                          (bind _returnvalue_3 (`KismetSystemLibrary.K2_SetTimerDelegate` (delegate `DamageEvent`) (`self.DamageDeltaSecond`) true))
                          (set `self.DamageTimer` _returnvalue_3))))
                    (:`else`)))))))))))

(event `DestroySphere`
  (bind _returnvalue (`self.GetAvatarActorFromActorInfo`))
  (`GameplayCueFunctionLibrary.ExecuteGameplayCueOnActor` _returnvalue (struct :`TagName` "GameplayCue.ElectroSphere.Destroy") (`AbilitySystemBlueprintLibrary.MakeGameplayCueParameters` 0.0 0.0 (struct) (struct) (struct) (struct) (struct) (0.0 0.0 0.0) (0.0 0.0 0.0) null (stale `self.K2_ActivateAbility` _electrosphere)))
  (`GameplayCueFunctionLibrary.RemoveGameplayCueOnActor` _returnvalue (struct :`TagName` "GameplayCue.ElectroSphere.Looping") (`AbilitySystemBlueprintLibrary.MakeGameplayCueParameters` 0.0))
  (`self.RemoveShockLoopStateAndCue`)
  (`self.K2_EndAbility`))

(event `self.K2_OnEndAbility`
  (params (bWasCancelled :type Boolean))
  (`KismetSystemLibrary.K2_ClearAndInvalidateTimerHandle` (`self.Timer`))
  (`KismetSystemLibrary.K2_ClearAndInvalidateTimerHandle` (`self.DamageTimer`))
  (`self.HideMagicCircleAndRangeIndicator`))

(event `DamageEvent`
  (for _array_element (`AuraElectroSphere.AdditionalOverlappingActors` (`self.ElectroSphere`))
    (`AuraAbilitySystemLibrary.ApplyDamageEffect` (`self.MakeDamageEffectParamsFromClassDefaults` _array_element))))

(fn `RemoveShockLoopCueFromAdditionalTargets`
  (params (`Dead Actor` :type "Actor Object Reference"))
  (set `self.Dead Actor` `Dead Actor`)
  (`GameplayCueFunctionLibrary.RemoveGameplayCueOnActor` (`self.Dead Actor`) (struct :`TagName` "GameplayCue.ShockLoop") (`AbilitySystemBlueprintLibrary.MakeGameplayCueParameters` 0.0)))

(fn `RemoveShockLoopStateAndCue`
  (for _array_element (`AuraElectroSphere.AdditionalOverlappingActors` (`self.ElectroSphere`))
    (message `CombatInterface.SetIsBeingShocked` _array_element false)
    (`self.RemoveShockLoopCueFromAdditionalTargets` _array_element))
  (`Actor.K2_DestroyActor` (`self.ElectroSphere`)))