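; BP_ElectroSphere is the lightning sphere actor for Aura's ElectroSphere ability, linking shock effects to targets around it.
; Each tick it calls DetectAdditionalTargets, defined outside this graph, with its owner in the array, and spins its mesh around yaw.
; AddShockLoopCueToTargets adds the looping shock GameplayCue on a given target, passing the sphere's root as the attach component.
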(event `self.ReceiveTick`
  (params (DeltaSeconds :type "Float (single-precision)"))
  (`self.DetectAdditionalTargets` (`|MakeArray` (`self.GetOwner`)))
  (`SceneComponent.K2_AddWorldRotation` (`self.Mesh`) (`KismetMathLibrary.MakeRotator` 0.0 0.0 (* DeltaSeconds -180.0)) false false))

(fn `AddShockLoopCueToTargets`
  (params (Target :type "Actor Object Reference"))
  (locals (TargetActor :type "Actor Object Reference"))
  (set `local.TargetActor` Target)
  (`GameplayCueFunctionLibrary.AddGameplayCueOnActor` (`local.TargetActor`) (struct :`TagName` "GameplayCue.ShockLoop") (`AbilitySystemBlueprintLibrary.MakeGameplayCueParameters` 0.0 0.0 (struct) (struct) (struct) (struct) (struct) (`self.K2_GetActorLocation` (`local.TargetActor`)) (0.0 0.0 0.0) null null (`local.TargetActor`) null 1 1 (`self.RootComponent`))))

(fn `UserConstructionScript`)