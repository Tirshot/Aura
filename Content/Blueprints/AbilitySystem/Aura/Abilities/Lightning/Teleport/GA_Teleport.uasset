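; Lightning teleport gameplay ability that moves Aura to the location under the mouse and knocks back those near the arrival point.
; It faces the target and plays a cast montage, whose gameplay event triggers the teleport and cue.
; Success spawns a ghost effect, applies radial damage, then commits cost, skipping cooldown when an upgrade check grants a reset.
; Ending the ability stops the player controller's auto-run.
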(event `self.K2_ActivateAbility`
  (bind _returnvalue (`self.GetAvatarActorFromActorInfo`))
  (bind _returnvalue_2 (`self.GetAvatarActorFromActorInfo`))
  (bind (_returnvalue_x _returnvalue_y _returnvalue_z) (`KismetMathLibrary.BreakVector` (`Actor.K2_GetActorLocation` _returnvalue_2)))
  (bind _asbp_aura_character (cast `/Game/Blueprints/Character/Aura/BP_AuraCharacter` _returnvalue_2))
  (set `self.InitialLocation` (`KismetMathLibrary.MakeVector` _returnvalue_x _returnvalue_y (- _returnvalue_z (`CapsuleComponent.GetScaledCapsuleHalfHeight` (`Character.CapsuleComponent` _asbp_aura_character)))))
  (bind (_asynctaskproxy _datahandle) (`TargetDataUnderMouse.CreateTargetDataUnderMouse`)
    (:`ValidData`
      (set `self.HitResult` (`AbilitySystemBlueprintLibrary.GetHitResultFromTargetData` _datahandle))
      (bind _output_get (set `self.Destination` (`.Location` (`GameplayStatics.BreakHitResult` (`self.HitResult`)))))
      (message `CombatInterface.UpdateFacingTarget` (`self.GetAvatarActorFromActorInfo`) _output_get)
      (`AbilityTask_PlayMontageAndWait.CreatePlayMontageAndWaitProxy` "None" "/Game/Assets/Characters/Aura/Animations/Abilities/AM_Cast_Teleport.AM_Cast_Teleport"
        (:`then`
          (`GameplayCueFunctionLibrary.ExecuteGameplayCueOnActor` (`self.GetAvatarActorFromActorInfo`) (struct :`TagName` "GameplayCue.Cast.Teleport") (`AbilitySystemBlueprintLibrary.MakeGameplayCueParameters` 0.0 0.0 (struct) (struct) (struct) (struct) (struct) (`self.InitialLocation`)))
          (`AbilityTask_WaitGameplayEvent.WaitGameplayEvent` (struct :`TagName` "Montage.Teleport") null true
            (:`EventReceived`
              (bind _returnvalue_3 (`self.TeleportToLocation` (`self.HitResult`)))
              (`GameplayCueFunctionLibrary.ExecuteGameplayCueOnActor` (`self.GetAvatarActorFromActorInfo`) (struct :`TagName` "GameplayCue.Teleport") (`AbilitySystemBlueprintLibrary.MakeGameplayCueParameters` 0.0 0.0 (struct) (struct) (struct) (struct) (struct) (+ (`self.Destination`) (0.0 0.0 80.0))))
              (if _returnvalue_3
                (`self.GhostEffect` (`self.InitialLocation`) (`self.Destination`) "/Game/Blueprints/Actor/BP_GhostEffectActor.BP_GhostEffectActor_C" "/Game/Kobo_Dungeon/Materials/M-FX/M-Embers.M-Embers")
                (bind _outoverlappingactors (`AuraAbilitySystemLibrary.GetLivePlayersWithinRadius` _returnvalue (`|MakeArray` _returnvalue) 500.0 (`self.Destination`)))
                (for _array_element _outoverlappingactors
                  (bind _return_value (`self.CalculateKnockBackDirection` _array_element))
                  (`AuraAbilitySystemLibrary.ApplyDamageEffect` (`self.MakeDamageEffectParamsFromClassDefaults` _array_element (`self.Destination`) false _return_value true _return_value)))
                (`self.CheckAbilityUpgrades` (struct :`TagName` "Abilities.Lightning.Teleport"))
                (bind _returnvalue_4 (`self.ShouldTeleportCooldownReset`))
                (if _returnvalue_4
                  (`self.K2_CommitAbilityCost` false)
                  (else
                    (`self.K2_CommitAbility`)))
                (`self.K2_EndAbility`)
                (else
                  (`self.K2_EndAbility`))))))))))

(event `self.K2_OnEndAbility`
  (params (bWasCancelled :type Boolean))
  (bind _asaura_character (cast `AuraCharacter` (`self.GetAvatarActorFromActorInfo`)))
  (bind _asaura_player_controller (cast `AuraPlayerController` (`Pawn.GetController` _asaura_character)))
  (`AuraPlayerController.StopAutoRun` _asaura_player_controller))

(fn `CalculateKnockBackDirection`
  (params (Target :type "Actor Object Reference"))
  (returns (`Return Value` :type "Vector Structure"))
  (return (- (`Actor.K2_GetActorLocation` Target) (`Actor.K2_GetActorLocation` (`self.GetAvatarActorFromActorInfo`)))))

(fn `새 함수`)