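; BP_FireBall is a FireBlast ability projectile that flies outward, returns to its ReturnToActor and explodes on arrival.
; On authority, one timeline lerps it along its forward vector to an apex, then a second lerps it back toward the actor's live location.
; Within ExplodeDistance it calls OnHit, applies radial damage with knockback and death impulse to nearby non-friendly live players, then destroys itself.
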(event `self.ReceiveBeginPlay`)

(event `self.StartOutgoingTimeline`
  (bind (_returnvalue_roll _returnvalue_pitch _returnvalue_yaw) (`KismetMathLibrary.BreakRotator` (`KismetMathLibrary.MakeRotFromX` (`self.KnockbackDirection`))))
  (bind _array (`|MakeArray` (`self.GetOwner`)))
  (`/Engine/EditorBlueprintResources/ActorMacros.Switch Has Authority`
    (:`Authority`
      (set `self.InitialLocation` (`self.K2_GetActorLocation`))
      (set `self.ApexLocation` (+ (`self.InitialLocation`) (* (`self.GetActorForwardVector`) (`self.TravelDistance`))))
      (bind (_direction _outgoingtrack) (`Timeline|OutgoingTimeline`)
        (:`Update`
          (`self.K2_SetActorLocation` (`KismetMathLibrary.VLerp` (`self.InitialLocation`) (`self.ApexLocation`) _outgoingtrack)))
        (:`Finished`
          (bind (_direction_2 _outgoingtrack_2) (`Timeline|타임라인`)
            (:`Update`
              (`self.K2_SetActorLocation` (`KismetMathLibrary.VLerp` (`self.ApexLocation`) (`self.K2_GetActorLocation` (`self.ReturnToActor`)) _outgoingtrack_2))
              (if (`self.IsWithinExplodeDistance`)
                (`self.OnHit`)
                (`AuraAbilitySystemLibrary.SetIsRadialDamageEffectParam` (`self.ExplosionDamageParams`) true (`self.K2_GetActorLocation`) (`self.RadialDamageInnerRadius`) (`self.RadialDamageOuterRadius`))
                (`KismetArrayLibrary.Array_Add` _array self)
                (bind _outoverlappingactors (`AuraAbilitySystemLibrary.GetLivePlayersWithinRadius` self _array (`self.RadialDamageOuterRadius`) (`self.K2_GetActorLocation`)))
                (bind _output_get (set `self.OverlappingPlayers` _outoverlappingactors))
                (for _array_element _output_get
                  (if (`AuraAbilitySystemLibrary.IsNotFriend` _array_element (`self.GetOwner`))
                    (`AuraAbilitySystemLibrary.SetEffectParamsTargetAbilitySystemComponent` (`self.ExplosionDamageParams`) (`AbilitySystemBlueprintLibrary.GetAbilitySystemComponent` _array_element))
                    (set `self.KnockbackDirection` (- (`self.K2_GetActorLocation` _array_element) (`self.K2_GetActorLocation`)))
                    (`AuraAbilitySystemLibrary.SetKnockbackDirection` (`self.ExplosionDamageParams`) (`KismetMathLibrary.GetForwardVector` (`KismetMathLibrary.MakeRotator` _returnvalue_roll 0.0 _returnvalue_yaw)) (`self.KnockbackMagnitude`))
                    (`AuraAbilitySystemLibrary.SetDeathImpulseDirection` (`self.ExplosionDamageParams`) (`self.KnockbackDirection`) (`self.DeathImpulseMagnitude`))
                    (`AuraAbilitySystemLibrary.ApplyDamageEffect` (`self.ExplosionDamageParams`))))
                (`self.K2_DestroyActor`)))))))))

(fn `IsWithinExplodeDistance`
  (returns (ReturnValue :type Boolean))
  (return (<= (`KismetMathLibrary.VSize` (- (`self.K2_GetActorLocation`) (`self.K2_GetActorLocation` (`self.ReturnToActor`)))) (`self.ExplodeDistance`))))

(fn `UserConstructionScript`)