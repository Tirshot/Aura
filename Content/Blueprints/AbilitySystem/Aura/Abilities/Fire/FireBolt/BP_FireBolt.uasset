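; Firebolt projectile actor for the Aura fire ability, with visuals or audio delegated to a gameplay cue.
; On begin play it adds the Firebolt cue on its owner, attached to the bolt's root component, and removes it when destroyed.
; Sphere collision switches to query-only after a brief delay.
; Each tick compares movement with the last frame and destroys the bolt once it travels no more than a minimum distance.
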(event `self.ReceiveDestroyed`
  (`GameplayCueFunctionLibrary.RemoveGameplayCueOnActor` (`self.GetOwner`) (struct :`TagName` "GameplayCue.Firebolt") (`self.CueParams`)))

(event `self.ReceiveBeginPlay`
  (bind _returnvalue (`AbilitySystemBlueprintLibrary.MakeGameplayCueParameters` 0.0 0.0 (struct) (struct) (struct) (struct) (struct) (0.0 0.0 0.0) (0.0 0.0 0.0) null null null null 1 1 (`self.RootComponent`)))
  (`GameplayCueFunctionLibrary.AddGameplayCueOnActor` (`self.GetOwner`) (struct :`TagName` "GameplayCue.Firebolt") _returnvalue)
  (set `self.CueParams` _returnvalue)
  (`KismetSystemLibrary.Delay` 0.1)
  (bind _sphere (`self.Sphere`)
    (:`then`
      (`PrimitiveComponent.SetCollisionEnabled` _sphere "QueryOnly"))
    (:`else`)))

(event `self.ReceiveTick`
  (params (DeltaSeconds :type "Float (single-precision)"))
  (set `self.LocationLastFrame` (`self.LocationThisFrame`))
  (set `self.LocationThisFrame` (`self.K2_GetActorLocation`))
  (if (<= (`KismetMathLibrary.VSize` (- (`self.LocationThisFrame`) (`self.LocationLastFrame`))) (`self.MinDistancePerFrame`))
    (`self.K2_DestroyActor`)))

(fn `UserConstructionScript`)