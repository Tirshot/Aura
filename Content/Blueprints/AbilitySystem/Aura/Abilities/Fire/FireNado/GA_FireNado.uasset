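; GA_FireNado is a player fire ability that spawns a tornado at a mouse-targeted ground location.
; Activation shows a magic circle and stops auto-run, then an input press captures the target, updates motion-warp facing and plays the cast montage.
; The montage's gameplay event spawns the tornado, commits cost, hides the circle and starts a lifetime timer.
; When the timer expires, the tornado is destroyed with a sound, and only then is cooldown committed.
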(event `self.K2_ActivateAbility`
  (bind _returnvalue (`self.GetAvatarActorFromActorInfo`))
  (bind _returnvalue_2 (`self.GetAvatarActorFromActorInfo`))
  (`|ExecutionSequence`
    (:`then_0`
      ;[1 1 1] 범위 지정 데칼 Show
      (message `PlayerInterface.ShowMagicCircle` _returnvalue null)
      ;[1 1 1] 자동 이동 중지
      (bind _asaura_character (cast `AuraCharacter` _returnvalue))
      (bind _asaura_player_controller (cast `AuraPlayerController` (`Pawn.GetController` _asaura_character)))
      (`AuraPlayerController.StopAutoRun` _asaura_player_controller)
      (`GameplayCueFunctionLibrary.ExecuteGameplayCueOnActor` (`self.GetAvatarActorFromActorInfo`) (struct :`TagName` "GameplayCue.Message.WaitForExecute") (`AbilitySystemBlueprintLibrary.MakeGameplayCueParameters` 0.0 0.0 (struct) (struct) (struct :`TagName` "GameplayCue.Message.WaitForExecute"))))
    (:`then_1`
      (`AbilityTask_WaitInputPress.WaitInputPress` false
        (:`OnPress`
          (bind (_asynctaskproxy _datahandle) (`TargetDataUnderMouse.CreateTargetDataUnderMouse`)
            (:`ValidData`
              (set `self.MouseLocation` (`.ImpactPoint` (`GameplayStatics.BreakHitResult` (`AbilitySystemBlueprintLibrary.GetHitResultFromTargetData` _datahandle))))
              ;[1 1 1] 모션 워핑
              (message `CombatInterface.UpdateFacingTarget` (`self.GetAvatarActorFromActorInfo`) (`self.MouseLocation`))
              (`AbilityTask_PlayMontageAndWait.CreatePlayMontageAndWaitProxy` "None" "/Game/Assets/Characters/Aura/Animations/Abilities/AM_Cast_FireNado.AM_Cast_FireNado"
                (:`then`
                  (`AbilityTask_WaitGameplayEvent.WaitGameplayEvent` (struct :`TagName` "Abilities.Fire.Firenado") null true
                    (:`EventReceived`
                      (bind _returnvalue_3 (`self.SpawnTornadoToLocation` (`self.MouseLocation`)))
                      (bind _output_get (set `self.FireTornado` _returnvalue_3))
                      (`self.K2_CommitAbilityCost` false)
                      (`Actor.K2_SetActorLocation` _output_get (`self.MouseLocation`) false true)
                      (bind _returnvalue_4 (`KismetSystemLibrary.K2_SetTimerDelegate` (delegate `DestroyTornado`) (`self.SpawnTime`)))
                      (set `self.Timer` _returnvalue_4)
                      (message `PlayerInterface.HideMagicCircle` _returnvalue_2)
                      (`self.RemoveRangeSpellHelpMessage` _returnvalue_2))))
                (:`OnInterrupted`
                  (`self.K2_EndAbility` :!label _label))
                (:`OnCancelled`
                  (goto _label))))))))))

(event `DestroyTornado`
  (`GameplayStatics.PlaySoundAtLocation` "/Game/Assets/Sounds/Abilities/FireNado/sfx_FireNado_End.sfx_FireNado_End" (`Actor.K2_GetActorLocation` (`self.FireTornado`)) (struct) 1.0 1.0 0.0 null null null null)
  (`Actor.K2_DestroyActor` (`self.FireTornado`))
  (`self.K2_CommitAbilityCooldown` false)
  (`self.K2_EndAbility`))

(event `self.K2_OnEndAbility`
  (params (bWasCancelled :type Boolean))
  (`parent.K2_OnEndAbility` bWasCancelled)
  (if bWasCancelled
    (message `PlayerInterface.HideMagicCircle` (`self.GetAvatarActorFromActorInfo`)))
  (bind _asaura_character (cast `AuraCharacter` (`self.GetAvatarActorFromActorInfo`)))
  (bind _asaura_player_controller (cast `AuraPlayerController` (`Pawn.GetController` _asaura_character)))
  (`AuraPlayerController.StopAutoRun` _asaura_player_controller)
  (`KismetSystemLibrary.K2_ClearAndInvalidateTimerHandle` (`self.Timer`)))