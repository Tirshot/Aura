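; Gameplay ability for the Arcane Shards spell, which spawns shards at a ground-targeted location chosen with the mouse.
; On activation it shows a magic circle and range indicator, then waits for a press to capture target data under the mouse.
; It then turns the avatar for motion warping, checks upgrades, creates a point collection and plays the cast montage.
; The montage's gameplay event triggers the shard spawn.
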(event `self.K2_ActivateAbility`
  (`self.ShowMagicCircle` (`self.RadialDamageOuterRadius`))
  (`self.ShowRangeIndicator` "ERS_Circle" 50.0)
  ;[1 1 1] 마우스 위치 가져오기
  (`AbilityTask_WaitInputPress.WaitInputPress` false
    (:`OnPress`
      (bind (_asynctaskproxy _datahandle) (`TargetDataUnderMouse.CreateTargetDataUnderMouse`)
        (:`ValidData`
          (`|ExecutionSequence`
            (:`then_0`
              (`self.ReceivedMouseHitResult` _datahandle)
              ;[1 1 1] 모션 워핑
              (`self.HideMagicCircleAndRangeIndicator`)
              (message `CombatInterface.UpdateFacingTarget` (`self.GetAvatarActorFromActorInfo`) (`self.CurrentTargetLocation`))
              (`self.CheckAbilityUpgrades`)
              (`self.CreatePointCollection`))
            (:`then_1`
              ;[1 1 1] 몽타주 재생 대기
              (`AbilityTask_PlayMontageAndWait.CreatePlayMontageAndWaitProxy` "None" "/Game/Assets/Characters/Aura/Animations/Abilities/AM_Cast_ArcaneShards_Short.AM_Cast_ArcaneShards_Short" 1.0 "None" false
                (:`then`
                  (`AbilityTask_WaitGameplayEvent.WaitGameplayEvent` (struct :`TagName` "Event.Montage.ArcaneShards") null true
                    (:`EventReceived`
                      (`self.ReadyToSpawnShards`))))))))))))