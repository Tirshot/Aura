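; Magic circle actor for the Arcane Shards ability, shown as a slowly spinning decal that highlights actors inside its box.
; Its CircleInitialized event executes a message-tagged gameplay cue on the avatar, and RemoveCircle removes that message through the avatar's Aura ability system component.
; Tick rotates the decal, while box overlap begin and end send highlight and unhighlight messages to the overlapping actor.
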(event `self.ReceiveBeginPlay`
  (add `self.CircleInitialized` (delegate `CircleInitialized_이벤트`))
  (add `self.RemoveCircle` (delegate `RemoveCircle_이벤트`)))

(event `CircleInitialized_이벤트` :!signature `self.CircleInitialized`
  (params (AvatarActor :type "Actor Object Reference"))
  (`GameplayCueFunctionLibrary.ExecuteGameplayCueOnActor` AvatarActor (`self.Gameplay Cue Tag`) (`AbilitySystemBlueprintLibrary.MakeGameplayCueParameters` 0.0 0.0 (struct) (struct) (struct :`TagName` "GameplayCue.Message.WaitForExecute"))))

(event `RemoveCircle_이벤트` :!signature `self.RemoveCircle`
  (params (AvatarActor :type "Actor Object Reference"))
  (bind _asaura_ability_system_component (cast `AuraAbilitySystemComponent` (`AbilitySystemBlueprintLibrary.GetAbilitySystemComponent` AvatarActor)))
  (`AuraAbilitySystemComponent.MessageRemove` _asaura_ability_system_component (`self.Gameplay Cue Tag`)))

(event `self.ReceiveTick`
  (params (DeltaSeconds :type "Float (single-precision)"))
  (`|ExecutionSequence`
    (:`then_0`
      (`SceneComponent.K2_AddLocalRotation` (`self.MagicCircleDecal`) (`KismetMathLibrary.MakeRotator` (* DeltaSeconds 8.0)) false false))))

(event `self.Box.OnComponentBeginOverlap`
  (params (OverlappedComponent :type "PrimitiveComponent Object Reference") (OtherActor :type "Actor Object Reference") (OtherComp :type "PrimitiveComponent Object Reference") (OtherBodyIndex :type Integer) (bFromSweep :type Boolean) (SweepResult :type "HitResult Structure (by ref)"))
  (message `HighlightInterface.HighlightActor` OtherActor))

(event `self.Box.OnComponentEndOverlap`
  (params (OverlappedComponent :type "PrimitiveComponent Object Reference") (OtherActor :type "Actor Object Reference") (OtherComp :type "PrimitiveComponent Object Reference") (OtherBodyIndex :type Integer))
  (message `HighlightInterface.UnHighlightActor` OtherActor))

(fn `UserConstructionScript`)