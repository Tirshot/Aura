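; Mind control gameplay ability that temporarily turns the combat target under the mouse into a Player-tagged ally.
; A cast montage and gameplay event trigger the actor tag swap and looping cue, cancelling on targets already tagged Player.
; A timer then restores the Enemy tag, removes the cue and ends the ability.
; The timer is hardcoded to three seconds; the computed MindControlDuration value is unused.
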(event `self.K2_ActivateAbility`
  (bind (_asynctaskproxy _datahandle) (`TargetDataUnderMouse.CreateTargetDataUnderMouse`)
    (:`ValidData`
      (bind (_bblockinghit _binitialoverlap _time _distance _location _impactpoint _normal _impactnormal _physmat _hitactor) (`GameplayStatics.BreakHitResult` (`AbilitySystemBlueprintLibrary.GetHitResultFromTargetData` _datahandle)))
      (if _bblockinghit
        (set `self.TargetActor` _hitactor)
        (set `self.TargetLocation` _location)
        (message `CombatInterface.UpdateFacingTarget` (`self.GetAvatarActorFromActorInfo`) (`self.TargetLocation`))
        (`AbilityTask_PlayMontageAndWait.CreatePlayMontageAndWaitProxy` "None" "/Game/Assets/Characters/Aura/Animations/Abilities/AM_Cast_MindControl.AM_Cast_MindControl"
          (:`then`
            (`AbilityTask_WaitGameplayEvent.WaitGameplayEvent` (struct :`TagName` "Abilities.Arcane.MindControl") null true
              (:`then`
                (cast `CombatInterface` (`self.TargetActor`)
                  (:`CastFailed`
                    (`self.K2_CancelAbility`))))
              (:`EventReceived`
                (`|ExecutionSequence`
                  (:`then_0`
                    (`self.SetOriginalTag` (`self.TargetActor`)))
                  (:`then_1`
                    (bind _returnvalue (`self.GetScalableFloatToFloat` (`self.MindControlDuration`)))
                    (set `self.MindControlDurationFloat` _returnvalue))
                  (:`then_2`
                    (if (`Actor.ActorHasTag` (`self.TargetActor`) "Player")
                      (`self.K2_CancelAbility` :!label _label)))
                  (:`then_3`
                    (bind _returnvalue_2 (`self.ChangeActorTag` (`self.TargetActor`) "Player"))
                    (if _returnvalue_2
                      (bind _output_get (set `self.CueParams` (`AbilitySystemBlueprintLibrary.MakeGameplayCueParameters` 0.0 0.0 (struct) (struct) (struct) (struct) (struct) (`Actor.K2_GetActorLocation` (`self.TargetActor`)) (0.0 0.0 0.0) null null null null 1 1 (`Actor.GetComponentByClass` (`self.TargetActor`) "/Script/Engine.CapsuleComponent"))))
                      (`GameplayCueFunctionLibrary.AddGameplayCueOnActor` (`self.TargetActor`) (struct :`TagName` "GameplayCue.MindControl") _output_get)
                      (if true
                        (`/Engine/EditorBlueprintResources/StandardMacros.IsValid` (`self.TargetActor`)
                          (:`Is Valid`
                            (bind _returnvalue_3 (`KismetSystemLibrary.K2_SetTimerDelegate` (delegate `Control`) 3.0))
                            (set `self.TimerHandle` _returnvalue_3)
                            (`self.K2_CommitAbility`))
                          (:`Is Not Valid`
                            (`self.K2_EndAbility` :!label _label_2)))
                        (else
                          (goto _label_2)))
                      (else
                        (goto _label)))))))))
        (else
          (`self.K2_EndAbility`))))))

(event `self.K2_OnEndAbility`
  (params (bWasCancelled :type Boolean))
  (`KismetSystemLibrary.K2_ClearAndInvalidateTimerHandle` (`self.TimerHandle`)))

(event `Control`
  (`self.ChangeActorTag` (`self.TargetActor`) "Enemy")
  (`GameplayCueFunctionLibrary.RemoveGameplayCueOnActor` (`self.TargetActor`) (struct :`TagName` "GameplayCue.MindControl") (`self.CueParams`))
  (`self.K2_EndAbility`))