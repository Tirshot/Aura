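; BP_Aura_MainMenu is the main menu scene actor that sets up the menu and animates its fireball and magic circle.
; On BeginPlay it plays menu music, adds WBP_MainMenu to the viewport with UI-only input and a visible cursor, and caches the fireball's starting location.
; Each Tick advances a timer wrapped at 2π to bob the Niagara fireball along a sine wave, and spins the magic circle decal at a configurable rate.
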(event `self.ReceiveBeginPlay`
  (bind _returnvalue (`GameplayStatics.GetPlayerController` 0))
  (set `self.FireBallInitialLocation` (`SceneComponent.K2_GetComponentLocation` (`self.Niagara`)))
  (`GameplayStatics.PlaySound2D` "/Game/Assets/Sounds/Music/Music_MainMenu.Music_MainMenu" 1.0 1.0 0.0 null null)
  (bind _returnvalue_2 (`|CreateWidget` "/Game/Blueprints/UI/MainMenu/WBP_MainMenu.WBP_MainMenu_C"))
  (`UserWidget.AddToViewport` _returnvalue_2 0)
  (`WidgetBlueprintLibrary.SetInputMode_UIOnlyEx` _returnvalue _returnvalue_2)
  (set `PlayerController.bShowMouseCursor` true _returnvalue))

(event `self.ReceiveTick`
  (params (DeltaSeconds :type "Float (single-precision)"))
  (`self.Update Time` DeltaSeconds)
  (`self.UpdateFireBallUpAndDown`)
  (`self.UpdateDecalRotation`))

(fn `Update Time`
  (params (DeltaSeconds :type "Float (double-precision)"))
  (bind _output_get (set `self.Time` (+ DeltaSeconds (`self.Time`))))
  (if (> _output_get (`KismetMathLibrary.MultiplyByPi` 2.0))
    (set `self.Time` 0.0)))

(fn `UpdateDecalRotation`
  (`SceneComponent.K2_AddLocalRotation` (`self.Decal`) (`KismetMathLibrary.MakeRotator` (* (`GameplayStatics.GetWorldDeltaSeconds`) (`self.MagicCircleRotationRate`))) false false))

(fn `UpdateFireBallUpAndDown`
  (`SceneComponent.K2_SetWorldLocation` (`self.Niagara`) (+ (`self.FireBallInitialLocation`) (`KismetMathLibrary.MakeVector` 0.0 0.0 (* (`KismetMathLibrary.Sin` (`self.Time`)) (`self.Amplitude`)))) false false))

(fn `UserConstructionScript`)