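; Director Blueprint for the Dungeon5 level sequence, handling player state around the cinematic.
; One sequencer event hides the Aura HUD overlay, makes the player invincible through BP_AuraGameMode and disables movement.
; The other restores the overlay and walking movement, then starts a timer that removes invincibility after InvincibleTime, leaving a grace period once control returns.
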(event `self.OnCreated`)

(event `SequenceEvent`
  (`self.HideOverlay`)
  (bind _asbp_aura_game_mode (cast `/Game/Blueprints/Game/BP_AuraGameMode` (`GameplayStatics.GetGameMode`)))
  (`AuraGameModeBase.OnSetActorInvincible` _asbp_aura_game_mode (`GameplayStatics.GetPlayerCharacter` 0) true)
  (`CharacterMovementComponent.SetMovementMode` (`Character.CharacterMovement` (`GameplayStatics.GetPlayerCharacter` 0)) "MOVE_None" 0))

(event `SequenceEvent_0`
  (`self.ShowOverlay`)
  (`KismetSystemLibrary.K2_SetTimerDelegate` (delegate `SetInvincible`) (`self.InvincibleTime`))
  (`CharacterMovementComponent.SetMovementMode` (`Character.CharacterMovement` (`GameplayStatics.GetPlayerCharacter` 0)) "MOVE_Walking" 0))

(event `SetInvincible`
  (bind _asbp_aura_game_mode (cast `/Game/Blueprints/Game/BP_AuraGameMode` (`GameplayStatics.GetGameMode`)))
  (`AuraGameModeBase.OnSetActorInvincible` _asbp_aura_game_mode (`GameplayStatics.GetPlayerCharacter` 0) false))

(fn `HideOverlay`
  (bind _asbp_aura_hud (cast `/Game/Blueprints/UI/HUD/BP_AuraHUD` (`PlayerController.GetHUD` (`GameplayStatics.GetPlayerController` 0))))
  (`AuraHUD.HideOverlay` _asbp_aura_hud))

(fn `ShowOverlay`
  (bind _asbp_aura_hud (cast `/Game/Blueprints/UI/HUD/BP_AuraHUD` (`PlayerController.GetHUD` (`GameplayStatics.GetPlayerController` 0))))
  (`AuraHUD.ShowOverlay` _asbp_aura_hud))