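; BP_Boss_Shaman is the Shaman boss character, adding intro roar and berserk presentation to its parent class.
; When BP_AuraCharacter enters AIStartSphere, the boss plays its roar montage, then disables the sphere's collision once the montage ends.
; The berserk montage event swaps the mesh to a rage material and replays the roar.
; Health changes read a target from the Blackboard, but nothing visible uses it.
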(event `self.ReceiveBeginPlay`
  (`parent.ReceiveBeginPlay`)
  (set `self.BlackBoard` (`AIBlueprintHelperLibrary.GetBlackboard` null))
  (add `AuraEnemy.OnHealthChanged` (delegate `OnHealthChanged_이벤트`))
  (add `AuraBossMonster.OnBeginBerserkMontage` (delegate `OnBeginBerserkMontage_이벤트`)))

(event `OnHealthChanged_이벤트`
  (params (NewValue :type "Float (single-precision)"))
  ; 타격 대상 주목
  (bind _blackboard (`self.BlackBoard`)
    (:`then`
      (set `self.Target` (`BlackboardComponent.GetValueAsObject` _blackboard (`self.Key Name_0_0`))))
    (:`else`)))

(event `OnBeginBerserkMontage_이벤트`
  ; 광폭화
  (`self.SetMeshMaterialToRage`)
  (`|PlayMontage` (`self.Mesh`) "/Game/Assets/Enemies/Shaman/Animations/AM_Shaman_Roar.AM_Shaman_Roar"))

(event `self.ReceiveTick`
  (params (DeltaSeconds :type "Float (single-precision)")))

(event `self.SpawnLoot`
  (`parent.SpawnLoot`))

(event `self.AIStartSphere.OnComponentBeginOverlap`
  (params (OverlappedComponent :type "PrimitiveComponent Object Reference") (OtherActor :type "Actor Object Reference") (OtherComp :type "PrimitiveComponent Object Reference") (OtherBodyIndex :type Integer) (bFromSweep :type Boolean) (SweepResult :type "HitResult Structure (by ref)"))
  (cast `/Game/Blueprints/Character/Aura/BP_AuraCharacter` OtherActor)
  (`|PlayMontage` (`self.Mesh`) "/Game/Assets/Enemies/Shaman/Animations/AM_Shaman_Roar.AM_Shaman_Roar"
    (:`OnCompleted`
      _)
    (:`OnBlendOut`
      _)
    (:`OnInterrupted`
      _))
  (`PrimitiveComponent.SetCollisionEnabled` (`self.AIStartSphere`) "NoCollision"))

(fn `SetMeshMaterialToRage`
  (`PrimitiveComponent.SetMaterial` (`self.Mesh`) 0 "/Game/Assets/Enemies/Shaman/Materials/M_Shaman_Rage.M_Shaman_Rage"))

(fn `UserConstructionScript`
  (`parent.UserConstructionScript`))