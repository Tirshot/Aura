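; Base Blueprint for boss monsters, handling attack facing, death dissolve, loot drops and post-dissolve upgrade rewards.
; UpdateFacingTarget feeds a Motion Warping target, while timelines drive the Dissolve parameter on body and weapon materials.
; When the body dissolve finishes, each BP_AuraCharacter's controller gets a server call to create card selection.
; SpawnLoot gets loot from LootTiers, then a looping timer spawns items one by one around the boss, optionally overriding effect-actor levels.
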(event `CombatInterface.UpdateFacingTarget`
  (params (Target :type "Vector Structure (by ref)"))
  (`MotionWarpingComponent.AddOrUpdateWarpTargetFromLocation` (`self.MotionWarping`) "FacingTarget" Target))

(event `self.ReceiveBeginPlay`
  (`parent.ReceiveBeginPlay`))

(event `self.StartDissolveTimeline`
  (params (DynamicMaterialInstance :type "MaterialInstanceDynamic Object Reference"))
  (bind (_direction _dissolvetrack) (`Timeline|타임라인_0`)
    (:`Update`
      (`MaterialInstanceDynamic.SetScalarParameterValue` DynamicMaterialInstance "Dissolve" _dissolvetrack))
    (:`Finished`
      (`self.SpawnUpgradeCard`))))

(event `self.StartWeaponDissolveTimeline`
  (params (DynamicMaterialInstance :type "MaterialInstanceDynamic Object Reference"))
  (bind (_direction _weapon_dissolve) (`Timeline|타임라인`)
    (:`Update`
      (`MaterialInstanceDynamic.SetScalarParameterValue` DynamicMaterialInstance "Dissolve" _weapon_dissolve))))

(event `self.SpawnLoot`
  (`parent.SpawnLoot`)
  (bind _returnvalue (`AuraAbilitySystemLibrary.GetLootTiers` self))
  (`/Engine/EditorBlueprintResources/StandardMacros.IsValid` _returnvalue
    (:`Is Valid`
      (bind _returnvalue_2 (`LootTiers.GetLootItems` _returnvalue))
      (bind _output_get (set `self.LootItems` _returnvalue_2))
      (bind _returnvalue_3 (`self.GetLootRotator` _output_get))
      (set `self.LootRotations` _returnvalue_3)
      (set `self.SpawnLootCount` 0)
      (bind _returnvalue_4 (`KismetSystemLibrary.K2_SetTimerDelegate` (delegate `SpawnLootItem`) 0.1 true))
      (set `self.LootTimer` _returnvalue_4)
      (`self.SpawnLootItem`))))

(event `SpawnLootItem`
  (bind (_lootclass _blootleveloverride) (break `LootItem` (`|GetArrayItem` (`self.LootItems`) (`self.SpawnLootCount`))))
  (if (< (`self.SpawnLootCount`) (`KismetArrayLibrary.Array_Length` (`self.LootItems`)))
    (bind _spawntransform (`self.GetLootTransform` (`self.SpawnLootCount`)))
    (bind _returnvalue (`|SpawnActorFromClass` _lootclass _spawntransform "AlwaysSpawn" "MultiplyWithRoot" null null))
    ;[1 1 1] 효과 액터 레벨 오버라이드
    (bind _asaura_effect_actor (cast `AuraEffectActor` _returnvalue)
      (:`then`
        (`/Engine/EditorBlueprintResources/StandardMacros.IsValid` _asaura_effect_actor
          (:`Is Valid`
            (if _blootleveloverride
              (set `AuraEffectActor.ActorLevel` (`KismetMathLibrary.Conv_IntToDouble` (`self.Level`)) _asaura_effect_actor)))
          (:`Is Not Valid`
            _)))
      (:`CastFailed`
        _))
    (`/Engine/EditorBlueprintResources/StandardMacros.IncrementInt` (`self.SpawnLootCount`))
    (else
      (`KismetSystemLibrary.K2_ClearAndInvalidateTimerHandle` (`self.LootTimer`)))))

(fn `GetLootRotator`
  (params (TargetArray :type "Array of LootItem Structure (by ref)"))
  (returns (ReturnValue :type "Array of Rotator Structure"))
  (return (`AuraAbilitySystemLibrary.EvenlySpacedRotators` (`self.GetActorForwardVector`) (`KismetMathLibrary.Vector_Up`) 360.0 (+ (`KismetArrayLibrary.Array_Length` TargetArray) 1))))

(fn `GetLootTransform`
  (params (LootCount :type Integer))
  (returns (SpawnTransform :type "Transform Structure"))
  (bind _output (`|GetArrayItem` (`self.LootRotations`) LootCount))
  (return (`KismetMathLibrary.MakeTransform` (+ (* (`KismetMathLibrary.GetForwardVector` _output) (`self.SpawnDistance`)) (`self.K2_GetActorLocation`)) _output)))

(fn `SpawnUpgradeCard`
  (bind _outactors (`GameplayStatics.GetAllActorsOfClass` "/Game/Blueprints/Character/Aura/BP_AuraCharacter.BP_AuraCharacter_C"))
  (for _array_element _outactors
    (bind _asaura_player_controller (cast `AuraPlayerController` (`PlayerState.GetPlayerController` (`Pawn.PlayerState` _array_element))))
    (`AuraPlayerController.Server_CreateCardSelection` _asaura_player_controller _array_element)))

(fn `UserConstructionScript`)