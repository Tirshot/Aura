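; BP_Scarecrow is a boss character that roars when the player first enters its detection sphere.
; Roar start and end events notify listeners, and roar start also launches the linked mission actors unless berserk.
; Each mission's end applies a massive fire damage gameplay effect to the boss itself.
; Tick slowly eases the spring arm toward a fixed rotation, and a widget displays total received damage.
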(event `self.StartDissolveTimeline`
  (params (DynamicMaterialInstance :type "MaterialInstanceDynamic Object Reference"))
  (`parent.StartDissolveTimeline` DynamicMaterialInstance))

(event `self.ReceiveBeginPlay`
  (`parent.ReceiveBeginPlay`)
  (set `self.InitialCamRotation` (`SceneComponent.K2_GetComponentRotation` (`self.SpringArm`)))
  (for _array_element (`self.MissionActors`)
    (add `MissionActor.OnEndMissionDelegate` _array_element (delegate `OnEndMissionDelegate_이벤트`))))

(event `OnEndMissionDelegate_이벤트`
  (`AbilitySystemComponent.BP_ApplyGameplayEffectToSelf` :`self` (`AbilitySystemBlueprintLibrary.GetAbilitySystemComponent` null) :`GameplayEffectClass` "/Game/Blueprints/Actor/Area/GE_FireArea_MassiveDamage.GE_FireArea_MassiveDamage_C" :`Level` 1.0))

(event `self.ReceiveActorBeginOverlap`
  (params (OtherActor :type "Actor Object Reference"))
  (`parent.ReceiveActorBeginOverlap` OtherActor))

(event `self.ReceiveTick`
  (params (DeltaSeconds :type "Float (single-precision)"))
  (`parent.ReceiveTick` DeltaSeconds)
  (`SceneComponent.K2_SetWorldRotation` (`self.SpringArm`) (`KismetMathLibrary.RInterpTo` (`SceneComponent.K2_GetComponentRotation` (`self.SpringArm`)) (struct :`Pitch` -40.0 :`Yaw` -230.0) DeltaSeconds 0.3) false false))

(event `self.DetectSphere.OnComponentBeginOverlap`
  (params (OverlappedComponent :type "PrimitiveComponent Object Reference") (OtherActor :type "Actor Object Reference") (OtherComp :type "PrimitiveComponent Object Reference") (OtherBodyIndex :type Integer) (bFromSweep :type Boolean) (SweepResult :type "HitResult Structure (by ref)"))
  (cast `/Game/Blueprints/Character/Aura/BP_AuraCharacter` OtherActor)
  (`|PlayMontage` (`self.Mesh`) "/Game/Assets/Enemies/ScareCrow/AM_Scarecrow_RoarStart.AM_Scarecrow_RoarStart"
    (:`then`
      (clear `PrimitiveComponent.OnComponentBeginOverlap` (`self.DetectSphere`)))))

(event `self.OnRoarStart_BlueprintEvent`
  (`self.OnBossRoarStart`)
  (if (not (`self.bBerserk`))
    (for _array_element (`self.MissionActors`)
      (`MissionActor.StartMission` _array_element))))

(event `self.OnRoarEnd_BlueprintEvent`
  (`self.OnBossRoarEnd`))

(event `self.UpdateTotalReceivedDamageWidget`
  (params (TotalDamage :type "Float (single-precision)"))
  (bind _aswbp_received_damage (cast `/Game/Blueprints/UI/TotalReceivedDamage/WBP_ReceivedDamage` (`WidgetComponent.GetWidget` (`self.TotalReceivedDamageWidget`))))
  (`/Game/Blueprints/UI/TotalReceivedDamage/WBP_ReceivedDamage.UpdateTotalReceivedDamageWidget` _aswbp_received_damage TotalDamage))

(fn `UserConstructionScript`)